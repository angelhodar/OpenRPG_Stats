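; Actor component that manages an RPG character's attributes, including point spending, per-level growth, flat and percentage bonuses, and resets.
; Defaults come from a data table row unless save-slot data exists, and a debug check flags inconsistent rows.
; Recalculation derives final values, then applies or removes data-driven bonuses on the owner's BPC_Stats once per point of change.
; Events notify listeners and push values to registered widgets.
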(event `Initialize`
  (set `self.StatsComponent` (`Actor.GetComponentByClass` (`self.GetOwner`) "/Game/OpenRPG_Stats/Blueprints/Components/BPC_Stats.BPC_Stats_C"))
  (if (`self.DebugEnabled?`)
    (`self.CheckConsistency`))
  (bind _success_ (`self.LoadAttributes`))
  (if (not _success_)
    (`self.LoadAttributesTableData`))
  (`self.InitializeWidgets`))

(event `UpdateAttributePoints`
  (params (AvailablePoints :type Integer))
  ;[1 0.1647 0.1349] Attributes and Stats
  (for _array_element (`self.Widgets`)
    (message `/Game/OpenRPG_Stats/Blueprints/Interfaces/BPI_Attributes.UpdateDisplayedAttributePoints` _array_element AvailablePoints)))

(event `UpdateAttributeValue`
  (params (Attribute :type "/Game/OpenRPG_Stats/Enums/e_Attribute Enum" :default "NewEnumerator6") (NewValue :type Integer))
  ;[1 0.1647 0.1349] Attributes and Stats
  (for _array_element (`self.Widgets`)
    (message `/Game/OpenRPG_Stats/Blueprints/Interfaces/BPI_Attributes.UpdateDisplayedAttribute` _array_element Attribute NewValue)))

(event `UpdateStatValue`
  (params (Stat :type "/Game/OpenRPG_Stats/Enums/e_Stat Enum" :default "NewEnumerator7") (FinalValue :type "Float (double-precision)") (CurrentValue :type "Float (double-precision)"))
  ;[1 0.1647 0.1349] Attributes and Stats
  (for _array_element (`self.Widgets`)
    (message `/Game/OpenRPG_Stats/Blueprints/Interfaces/BPI_Stats.UpdateDisplayedStat` _array_element Stat FinalValue CurrentValue)))

(fn `AddAttributeBonuses`
  (params (AttributeBonuses :type "/Game/OpenRPG_Stats/Structs/s_AttributeBonus Structure"))
  (locals (LocalFlatBonuses :type "Map of /Game/OpenRPG_Stats/Enums/e_Attribute Enum to Float (double-precision)") (LocalPercentageBonuses :type "Map of /Game/OpenRPG_Stats/Enums/e_Attribute Enum to Float (double-precision)") (LocalCurrentLoopAttribute :type "/Game/OpenRPG_Stats/Enums/e_Attribute Enum") (LocalCurrentLoopAttributeData :type "/Game/OpenRPG_Stats/Structs/s_Attribute Structure"))
  (bind (_flatbonuses _percentagebonuses) (break `/Game/OpenRPG_Stats/Structs/s_AttributeBonus` AttributeBonuses))
  ;[0 0.8913 1] Adds the flat bonuses and percentage bonuses from the input struct s_AttributeBonuses to the attributes data. When its added it calls CalculateAtributesChangeOnStats, which calculates the final value for every attribute and apply scaled data from AttributeBonusesToStats map variable according to the new attribute values
  (set `local.LocalFlatBonuses` _flatbonuses)
  (set `local.LocalPercentageBonuses` _percentagebonuses)
  (bind _keys (`BlueprintMapLibrary.Map_Keys` (`local.LocalFlatBonuses`)))
  (for _array_element _keys
    (bind _output_get (set `local.LocalCurrentLoopAttribute` _array_element))
    (bind _output_get_2 (set `local.LocalCurrentLoopAttributeData` (`BlueprintMapLibrary.Map_Find` (`self.Attributes`) _output_get)))
    (bind _structout (setmembers `/Game/OpenRPG_Stats/Structs/s_Attribute` :`StructRef` _output_get_2 :`FlatBonuses` (+ (`.FlatBonuses_28_3F6008684D9845B3258C57AB96242FE5` (break `/Game/OpenRPG_Stats/Structs/s_Attribute` _output_get_2)) (`BlueprintMapLibrary.Map_Find` (`local.LocalFlatBonuses`) (`local.LocalCurrentLoopAttribute`)))))
    (`BlueprintMapLibrary.Map_Add` (`self.Attributes`) (`local.LocalCurrentLoopAttribute`) _structout))
  (bind _keys_2 (`BlueprintMapLibrary.Map_Keys` (`local.LocalPercentageBonuses`)))
  (for _array_element_2 _keys_2
    (bind _output_get_3 (set `local.LocalCurrentLoopAttribute` _array_element_2))
    (bind _output_get_4 (set `local.LocalCurrentLoopAttributeData` (`BlueprintMapLibrary.Map_Find` (`self.Attributes`) _output_get_3)))
    (bind _structout_2 (setmembers `/Game/OpenRPG_Stats/Structs/s_Attribute` :`StructRef` _output_get_4 :`PercentageBonuses` (+ (`.PercentageBonuses_29_4A36E47747DB8544BA56E4AF979B4155` (break `/Game/OpenRPG_Stats/Structs/s_Attribute` _output_get_4)) (`BlueprintMapLibrary.Map_Find` (`local.LocalPercentageBonuses`) (`local.LocalCurrentLoopAttribute`)))))
    (`BlueprintMapLibrary.Map_Add` (`self.Attributes`) (`local.LocalCurrentLoopAttribute`) _structout_2))
  (`self.CalculateAttributesFinalValues`)
  (return))

(fn `AddAttributeBonusesToStats`
  (params (Attribute :type "/Game/OpenRPG_Stats/Enums/e_Attribute Enum" :default "NewEnumerator6") (ReceivedPoints :type Integer))
  (locals (LocalAttribute :type "/Game/OpenRPG_Stats/Enums/e_Attribute Enum" :default "NewEnumerator6") (LocalPoints :type Integer) (LocalStatBonuses :type "/Game/OpenRPG_Stats/Structs/s_StatBonus Structure") (`LocalRemove?` :type Boolean))
  (bind (_value _returnvalue) (`BlueprintMapLibrary.Map_Find` (`.AttributeBonusesToStats_10_623131B64D373095975842BC34C25A8D` (break `/Game/OpenRPG_Stats/Structs/s_AttributesData` (`self.GetAttributesData`))) (`local.LocalAttribute`)))
  (set `local.LocalAttribute` Attribute)
  (bind _output_get (set `local.LocalPoints` ReceivedPoints))
  (`/Engine/EditorBlueprintResources/StandardMacros.CompareInt` _output_get
    (:`>`
      _)
    (:`==`
      (return))
    (:`<`
      (set `local.LocalRemove?` true)
      (set `local.LocalPoints` (`KismetMathLibrary.Abs_Int` (`local.LocalPoints`)))))
  (if _returnvalue
    (set `local.LocalStatBonuses` _value)
    (for _ (range (`local.LocalPoints`))
      (if (`local.LocalRemove?`)
        (`/Game/OpenRPG_Stats/Blueprints/Components/BPC_Stats.RemoveStatBonuses` (`self.StatsComponent`) (`local.LocalStatBonuses`))
        (else
          (`/Game/OpenRPG_Stats/Blueprints/Components/BPC_Stats.AddStatBonuses` (`self.StatsComponent`) (`local.LocalStatBonuses`)))))
    (return)
    (else
      (return))))

(fn `AddAttributesPerLevel`
  (locals (LocalCurrentLoopAttribute :type "/Game/OpenRPG_Stats/Enums/e_Attribute Enum") (LocalAttributesPerLevel :type "Map of /Game/OpenRPG_Stats/Enums/e_Attribute Enum to Object Object Reference"))
  (bind _output_get (set `local.LocalAttributesPerLevel` (`.AttributesPerLevel_15_EE2E70BF41ED7F6EF3231CBA9014991C` (break `/Game/OpenRPG_Stats/Structs/s_AttributesData` (`self.GetAttributesData`)))))
  (bind _keys (`BlueprintMapLibrary.Map_Keys` _output_get))
  (for _array_element _keys
    (bind _output_get_2 (set `local.LocalCurrentLoopAttribute` _array_element))
    (`self.AddPointsToAttribute` (`local.LocalCurrentLoopAttribute`) (`BlueprintMapLibrary.Map_Find` (`local.LocalAttributesPerLevel`) _output_get_2)))
  (return))

(fn `AddCustomWidgets`
  (params (Widgets :type "Array of UserWidget Object Reference"))
  (for _array_element Widgets
    (`KismetArrayLibrary.Array_AddUnique` (`self.Widgets`) _array_element))
  (return))

(fn `AddPointsToAttribute`
  (params (Attribute :type "/Game/OpenRPG_Stats/Enums/e_Attribute Enum" :default "NewEnumerator6") (Points :type Integer))
  (locals (LocalAttribute :type "/Game/OpenRPG_Stats/Enums/e_Attribute Enum") (LocalPoints :type Integer) (LocalAttributeData :type "/Game/OpenRPG_Stats/Structs/s_Attribute Structure"))
  (bind (_value _returnvalue) (`BlueprintMapLibrary.Map_Find` (`self.Attributes`) (`local.LocalAttribute`)))
  (set `local.LocalAttribute` Attribute)
  (bind _output_get (set `local.LocalPoints` Points))
  (if (!= _output_get 0)
    (if _returnvalue
      (bind _output_get_2 (set `local.LocalAttributeData` _value))
      (bind _structout (setmembers `/Game/OpenRPG_Stats/Structs/s_Attribute` :`StructRef` _output_get_2 :`BaseValue` (+ (`.BaseValue_5_5398D8464682C14444DF888899E8366F` (break `/Game/OpenRPG_Stats/Structs/s_Attribute` _output_get_2)) (`local.LocalPoints`))))
      (`BlueprintMapLibrary.Map_Add` (`self.Attributes`) (`local.LocalAttribute`) _structout)
      (`self.CalculateAttributesFinalValues`)
      (`self.AddAttributeBonusesToStats` (`local.LocalAttribute`) (`local.LocalPoints`))
      (return)
      (else
        (return)))
    (else
      (return))))

(fn `CalculateAttributesFinalValues`
  (locals (LocalCurrentLoopAttribute :type "/Game/OpenRPG_Stats/Enums/e_Attribute Enum") (LocalCurrentLoopAttributeData :type "/Game/OpenRPG_Stats/Structs/s_Attribute Structure") (LocalPreviousValue :type Integer) (LocalPreviousAttributeValues :type "Map of /Game/OpenRPG_Stats/Enums/e_Attribute Enum to /Game/OpenRPG_Stats/Structs/s_Attribute Structure"))
  (bind _localcurrentloopattribute (`local.LocalCurrentLoopAttribute`))
  (bind _localcurrentloopattribute_2 (`local.LocalCurrentLoopAttribute`))
  (set `local.LocalPreviousAttributeValues` (`self.Attributes`))
  (bind _keys (`BlueprintMapLibrary.Map_Keys` (`self.Attributes`)))
  (for _array_element _keys
    (bind _output_get (set `local.LocalCurrentLoopAttribute` _array_element))
    (bind _output_get_2 (set `local.LocalCurrentLoopAttributeData` (`BlueprintMapLibrary.Map_Find` (`self.Attributes`) _output_get)))
    (bind ((`BaseValue_5_5398D8464682C14444DF888899E8366F` _basevalue) (`FlatBonuses_28_3F6008684D9845B3258C57AB96242FE5` _flatbonuses) (`PercentageBonuses_29_4A36E47747DB8544BA56E4AF979B4155` _percentagebonuses)) (break `/Game/OpenRPG_Stats/Structs/s_Attribute` _output_get_2))
    (bind _output_get_3 (set `local.LocalPreviousValue` _basevalue))
    (bind _structout (setmembers `/Game/OpenRPG_Stats/Structs/s_Attribute` :`StructRef` _output_get_2 :`FinalValue` (+ _output_get_3 (`KismetMathLibrary.FTrunc` _flatbonuses) (`KismetMathLibrary.FTrunc` (/ (* _basevalue _percentagebonuses) 100.0)))))
    (`BlueprintMapLibrary.Map_Add` (`self.Attributes`) (`local.LocalCurrentLoopAttribute`) _structout)
    (`self.AddAttributeBonusesToStats` (`local.LocalCurrentLoopAttribute`) (- (`self.GetAttributeValue` (`local.LocalCurrentLoopAttribute`)) (`.FinalValue_9_4273F5764C3DF52F895994A4ED72F50D` (break `/Game/OpenRPG_Stats/Structs/s_Attribute` (`BlueprintMapLibrary.Map_Find` (`local.LocalPreviousAttributeValues`) (`local.LocalCurrentLoopAttribute`))))))
    (`self.UpdateAttributeValue` _localcurrentloopattribute (`self.GetAttributeValue` _localcurrentloopattribute))
    (`self.OnAttributeFinalValueChanged` _localcurrentloopattribute_2 (`local.LocalPreviousValue`) (`self.GetAttributeValue` _localcurrentloopattribute_2)))
  (return))

(fn `CheckConsistency`
  (locals (LocalDefaultAttributes :type "/Game/OpenRPG_Stats/Structs/s_AttributesData Structure") (LocalAttribute :type "/Game/OpenRPG_Stats/Enums/e_Attribute Enum"))
  (`/Engine/EditorBlueprintResources/StandardMacros.IsValid` (`self.AttributesTable`)
    (:`Is Valid`
      (bind _returnvalue (`|GetDataTableRow` (`self.AttributesTable`) (`self.AttributesTableRow`))
        (:`then`
          (bind _output_get (set `local.LocalDefaultAttributes` _returnvalue))
          (bind _keys (`BlueprintMapLibrary.Map_Keys` (`.AttributeBonusesToStats_10_623131B64D373095975842BC34C25A8D` (break `/Game/OpenRPG_Stats/Structs/s_AttributesData` _output_get))))
          (for _array_element _keys
            (bind _output_get_2 (set `local.LocalAttribute` _array_element))
            (if (not (`BlueprintMapLibrary.Map_Contains` (`.Attributes_16_BA76E1204E2CD013510F85AB363740DC` (break `/Game/OpenRPG_Stats/Structs/s_AttributesData` (`local.LocalDefaultAttributes`))) _output_get_2))
              (`KismetSystemLibrary.PrintString` (`KismetStringLibrary.Concat_StrStr` "Warning: Attribute " (`|GetEnumeratorNameAsString` (`local.LocalAttribute`)) " found in AttributeBonusesToStats but not in Attributes, clean that data!") true false (struct :`R` 1.0 :`G` 1.0 :`A` 1.0) 10.0)))
          (bind _keys_2 (`BlueprintMapLibrary.Map_Keys` (`.AttributesPerLevel_15_EE2E70BF41ED7F6EF3231CBA9014991C` (break `/Game/OpenRPG_Stats/Structs/s_AttributesData` (`local.LocalDefaultAttributes`)))))
          (for _array_element_2 _keys_2
            (bind _output_get_3 (set `local.LocalAttribute` _array_element_2))
            (if (not (`BlueprintMapLibrary.Map_Contains` (`.Attributes_16_BA76E1204E2CD013510F85AB363740DC` (break `/Game/OpenRPG_Stats/Structs/s_AttributesData` (`local.LocalDefaultAttributes`))) _output_get_3))
              (`KismetSystemLibrary.PrintString` (`KismetStringLibrary.Concat_StrStr` "Warning: Attribute " (`|GetEnumeratorNameAsString` (`local.LocalAttribute`)) " found in AttributesPerLevel but not in Attributes, clean that data!") true false (struct :`R` 1.0 :`G` 1.0 :`A` 1.0) 10.0)))
          (`KismetSystemLibrary.PrintString` "No errors found!" true false (struct :`G` 1.0 :`A` 1.0) 5.0)
          (return))
        (:`RowNotFound`
          (`KismetSystemLibrary.PrintString` (`KismetStringLibrary.Concat_StrStr` "AttributesTableRow " (`KismetStringLibrary.Conv_NameToString` (`self.AttributesTableRow`)) " not found in AttributesTable") true false (struct :`R` 1.0 :`A` 1.0) 10.0)
          (return))))
    (:`Is Not Valid`
      (`KismetSystemLibrary.PrintString` "Error: Not valid AttributesTable value assigned" true false (struct :`R` 1.0 :`A` 1.0) 10.0)
      (return))))

(fn `CreateAttributesSaveData`
  (returns (Data :type "/Game/OpenRPG_Stats/Structs/s_AttributesSaveData Structure"))
  (return (make `/Game/OpenRPG_Stats/Structs/s_AttributesSaveData` (`self.Attributes`) (`self.AvailableAttributePoints`) (`self.SpentAttributePoints`))))

(fn `GetAttributesData`
  (returns (Data :type "/Game/OpenRPG_Stats/Structs/s_AttributesData Structure"))
  (bind _returnvalue (`|GetDataTableRow` (`self.AttributesTable`) (`self.AttributesTableRow`))
    (:`then`
      (return _returnvalue))
    (:`RowNotFound`
      (return))))

(fn `GetAttributeValue`
  (params (Attribute :type "/Game/OpenRPG_Stats/Enums/e_Attribute Enum" :default "NewEnumerator6"))
  (returns (Value :type Integer))
  ;[0.02628 1 0.4395] Gets the calculated final value of the input attribute
  (return (`.FinalValue_9_4273F5764C3DF52F895994A4ED72F50D` (break `/Game/OpenRPG_Stats/Structs/s_Attribute` (`BlueprintMapLibrary.Map_Find` (`self.Attributes`) Attribute)))))

(fn `InitializeWidgets`
  (bind _keys (`BlueprintMapLibrary.Map_Keys` (`self.Attributes`)))
  (for _array_element _keys
    (`self.UpdateAttributeValue` _array_element (`self.GetAttributeValue` _array_element)))
  (`self.UpdateAttributePoints` (`self.AvailableAttributePoints`))
  (return))

(fn `LoadAttributes`
  (returns (`Success?` :type Boolean))
  (locals (LocalSavedData :type "/Game/OpenRPG_Stats/Structs/s_AttributesSaveData Structure"))
  (bind (_found_ _data) (`/Game/OpenRPG_Stats/Blueprints/SaveStats.GetAttributesData` (`self.StatsSaveObject`) (`self.SaveName`)))
  (bind _output_get (set `self.StatsSaveObject` (`/Game/OpenRPG_Stats/Blueprints/BPL_Stats.GetStatsSaveObject` (`self.StatsSaveSlot`))))
  (`/Engine/EditorBlueprintResources/StandardMacros.IsValid` _output_get
    (:`Is Valid`
      (if _found_
        (bind _output_get_2 (set `local.LocalSavedData` _data))
        (bind (_savedattributes _savedavailableattributepoints _savedspentattributepoints) (break `/Game/OpenRPG_Stats/Structs/s_AttributesSaveData` _output_get_2))
        (set `self.Attributes` _savedattributes)
        (set `self.AvailableAttributePoints` _savedavailableattributepoints)
        (set `self.SpentAttributePoints` _savedspentattributepoints)
        (return true)
        (else
          (return false))))
    (:`Is Not Valid`
      (return false))))

(fn `LoadAttributesTableData`
  (locals (LocalAttributesData :type "/Game/OpenRPG_Stats/Structs/s_AttributesData Structure") (LocalDefaultAttributes :type "Map of /Game/OpenRPG_Stats/Enums/e_Attribute Enum to Integer") (LocalAttribute :type "/Game/OpenRPG_Stats/Enums/e_Attribute Enum") (`LocalPreviousSuccess?` :type Boolean))
  (`/Engine/EditorBlueprintResources/StandardMacros.IsValid` (`self.AttributesTable`)
    (:`Is Valid`
      (bind _output_get (set `local.LocalDefaultAttributes` (`.Attributes_16_BA76E1204E2CD013510F85AB363740DC` (break `/Game/OpenRPG_Stats/Structs/s_AttributesData` (`self.GetAttributesData`)))))
      (bind _keys (`BlueprintMapLibrary.Map_Keys` _output_get))
      (for _array_element _keys
        (bind _output_get_2 (set `local.LocalAttribute` _array_element))
        (bind _value (`BlueprintMapLibrary.Map_Find` (`local.LocalDefaultAttributes`) _output_get_2))
        (`BlueprintMapLibrary.Map_Add` (`self.Attributes`) (`local.LocalAttribute`) (make `/Game/OpenRPG_Stats/Structs/s_Attribute` :`BaseValue` _value :`FinalValue` _value)))
      (return))
    (:`Is Not Valid`
      (return))))

(fn `ReceiveAttributePoints`
  (params (Points :type Integer))
  (locals (LocalPoints :type Integer))
  (bind _output_get (set `local.LocalPoints` Points))
  (bind _output_get_2 (set `self.AvailableAttributePoints` (+ _output_get (`self.AvailableAttributePoints`))))
  (`self.UpdateAttributePoints` _output_get_2)
  (`self.OnAttributePointsReceived` (`local.LocalPoints`) (`self.AvailableAttributePoints`))
  (return))

(fn `RemoveAttributeBonuses`
  (params (AttributeBonuses :type "/Game/OpenRPG_Stats/Structs/s_AttributeBonus Structure"))
  (locals (LocalFlatBonuses :type "Map of /Game/OpenRPG_Stats/Enums/e_Attribute Enum to Float (double-precision)") (LocalPercentageBonuses :type "Map of /Game/OpenRPG_Stats/Enums/e_Attribute Enum to Float (double-precision)") (LocalCurrentLoopAttribute :type "/Game/OpenRPG_Stats/Enums/e_Attribute Enum") (LocalCurrentLoopAttributeData :type "/Game/OpenRPG_Stats/Structs/s_Attribute Structure"))
  (bind (_flatbonuses _percentagebonuses) (break `/Game/OpenRPG_Stats/Structs/s_AttributeBonus` AttributeBonuses))
  ;[0 0.8913 1] Removes the flat bonuses and percentage bonuses from the input struct s_AttributeBonuses to the attributes data. When its added it calls CalculateAtributesChangeOnStats, which calculates the final value for every attribute and apply scaled data from AttributeBonusesToStats map variable according to the new attribute values
  (set `local.LocalFlatBonuses` _flatbonuses)
  (set `local.LocalPercentageBonuses` _percentagebonuses)
  (bind _keys (`BlueprintMapLibrary.Map_Keys` (`local.LocalFlatBonuses`)))
  (for _array_element _keys
    (bind _output_get (set `local.LocalCurrentLoopAttribute` _array_element))
    (bind _output_get_2 (set `local.LocalCurrentLoopAttributeData` (`BlueprintMapLibrary.Map_Find` (`self.Attributes`) _output_get)))
    (bind _structout (setmembers `/Game/OpenRPG_Stats/Structs/s_Attribute` :`StructRef` _output_get_2 :`FlatBonuses` (- (`.FlatBonuses_28_3F6008684D9845B3258C57AB96242FE5` (break `/Game/OpenRPG_Stats/Structs/s_Attribute` _output_get_2)) (`BlueprintMapLibrary.Map_Find` (`local.LocalFlatBonuses`) (`local.LocalCurrentLoopAttribute`)))))
    (`BlueprintMapLibrary.Map_Add` (`self.Attributes`) (`local.LocalCurrentLoopAttribute`) _structout))
  (bind _keys_2 (`BlueprintMapLibrary.Map_Keys` (`local.LocalPercentageBonuses`)))
  (for _array_element_2 _keys_2
    (bind _output_get_3 (set `local.LocalCurrentLoopAttribute` _array_element_2))
    (bind _output_get_4 (set `local.LocalCurrentLoopAttributeData` (`BlueprintMapLibrary.Map_Find` (`self.Attributes`) _output_get_3)))
    (bind _structout_2 (setmembers `/Game/OpenRPG_Stats/Structs/s_Attribute` :`StructRef` _output_get_4 :`PercentageBonuses` (- (`.PercentageBonuses_29_4A36E47747DB8544BA56E4AF979B4155` (break `/Game/OpenRPG_Stats/Structs/s_Attribute` _output_get_4)) (`BlueprintMapLibrary.Map_Find` (`local.LocalPercentageBonuses`) (`local.LocalCurrentLoopAttribute`)))))
    (`BlueprintMapLibrary.Map_Add` (`self.Attributes`) (`local.LocalCurrentLoopAttribute`) _structout_2))
  (`self.CalculateAttributesFinalValues`)
  (return))

(fn `ResetAttributes`
  (locals (LocalAttributesData :type "/Game/OpenRPG_Stats/Structs/s_AttributesData Structure") (LocalDefaultAttributes :type "Map of /Game/OpenRPG_Stats/Enums/e_Attribute Enum to Integer") (LocalCurrentLoopAttribute :type "/Game/OpenRPG_Stats/Enums/e_Attribute Enum"))
  (`/Engine/EditorBlueprintResources/StandardMacros.IsValid` (`self.AttributesTable`)
    (:`Is Valid`
      (bind _returnvalue (`|GetDataTableRow` (`self.AttributesTable`) (`self.AttributesTableRow`))
        (:`then`
          (bind _output_get (set `local.LocalAttributesData` _returnvalue))
          (bind _output_get_2 (set `local.LocalDefaultAttributes` (`.Attributes_16_BA76E1204E2CD013510F85AB363740DC` (break `/Game/OpenRPG_Stats/Structs/s_AttributesData` _output_get))))
          (bind _keys (`BlueprintMapLibrary.Map_Keys` _output_get_2))
          (for _array_element _keys
            (bind _output_get_3 (set `local.LocalCurrentLoopAttribute` _array_element))
            (`self.AddPointsToAttribute` (`local.LocalCurrentLoopAttribute`) (- (`BlueprintMapLibrary.Map_Find` (`local.LocalDefaultAttributes`) _output_get_3) (`.BaseValue_5_5398D8464682C14444DF888899E8366F` (break `/Game/OpenRPG_Stats/Structs/s_Attribute` (`BlueprintMapLibrary.Map_Find` (`self.Attributes`) (`local.LocalCurrentLoopAttribute`)))))))
          (`self.ReceiveAttributePoints` (`self.SpentAttributePoints`))
          (set `self.SpentAttributePoints` 0)
          (`self.OnAttributesResetted`)
          (return))
        (:`RowNotFound`
          (return))))
    (:`Is Not Valid`
      (return))))

(fn `SaveAttributes`
  (returns (`Success?` :type Boolean))
  (bind _output_get (set `self.StatsSaveObject` (`/Game/OpenRPG_Stats/Blueprints/BPL_Stats.GetStatsSaveObject` (`self.StatsSaveSlot`))))
  (`/Engine/EditorBlueprintResources/StandardMacros.IsValid` _output_get
    (:`Is Valid`
      (`/Game/OpenRPG_Stats/Blueprints/SaveStats.AddAtributesData` (`self.StatsSaveObject`) (`self.SaveName`) (`self.CreateAttributesSaveData`))
      (bind _returnvalue (`GameplayStatics.SaveGameToSlot` (`self.StatsSaveObject`) (`self.StatsSaveSlot`)))
      (return _returnvalue))
    (:`Is Not Valid`
      (return false))))

(fn `SpendAttributePoints`
  (params (Attribute :type "/Game/OpenRPG_Stats/Enums/e_Attribute Enum" :default "NewEnumerator6") (Points :type Integer))
  (locals (LocalAttribute :type "/Game/OpenRPG_Stats/Enums/e_Attribute Enum") (LocalPoints :type Integer))
  (bind _localattribute (`local.LocalAttribute`))
  ;[0.8861 1 0.09855] Called when the "+" button is pressed in the UI when there are available attribute points to spend. It calls AddPointsToAttribute which handles all the calculations and then adjusts the AvailableAttributePoints and SpentAttributePoints variables.
  (set `local.LocalAttribute` Attribute)
  (bind _output_get (set `local.LocalPoints` Points))
  (`self.AddPointsToAttribute` (`local.LocalAttribute`) _output_get)
  (set `self.AvailableAttributePoints` (- (`self.AvailableAttributePoints`) (`local.LocalPoints`)))
  (set `self.SpentAttributePoints` (+ (`self.SpentAttributePoints`) (`local.LocalPoints`)))
  (`self.UpdateAttributePoints` (`self.AvailableAttributePoints`))
  (`self.UpdateAttributeValue` _localattribute (`self.GetAttributeValue` _localattribute))
  (`self.OnAttributePointsSpent` (`local.LocalAttribute`) (`local.LocalPoints`) (`self.AvailableAttributePoints`))
  (return))
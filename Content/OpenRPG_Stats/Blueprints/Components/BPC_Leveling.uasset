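; Actor component for RPG leveling that tracks level and experience, with settings and rewards read from a data table row.
; Needed experience comes from a per-level map or an overridable custom formula.
; LevelUp grants attribute points through the owner's BPC_Attributes, while level and experience changes notify registered widgets and event listeners.
; Progress saves to and loads from a stats save slot by save name.
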(event Custom|ReceiveLevelUpReward
  (params (NewLevel :type Integer))
  (bind _levelrewards (Variables|Internal|GetLevelRewards))
  (bind (_value _returnvalue) (Utilities|Map|Find _levelrewards NewLevel))
  (if _returnvalue
    (Default|ReceiveAttributePoints (Variables|Default|GetAttributesComponent) (Utilities|Struct|Breaks_LevelUpReward _value))))

(event Custom|ExperienceFormula
  (params (NewLevel :type Integer))
  ;[0.7629 0.06718 1] Custom experience formula, this event will be called if you set the UseCustomExperienceFormula? boolean to true in the component Settings category. Here you have an example. Remember to always set the variable NeededExperience at the end of the calculations
  (Variables|General|SetNeededExperience (Math|Float|Truncate (|(((a*x)+(power(x,4)))+100) 5.0 (Math|Conversions|ToFloat(Integer) NewLevel)))))

(event Custom|Initialize
  (Variables|Default|SetStatsComponent (Actor|GetComponentbyClass (Components|GetOwner) "/Game/OpenRPG_Stats/Blueprints/Components/BPC_Stats.BPC_Stats_C"))
  (Variables|Default|SetAttributesComponent (Actor|GetComponentbyClass (Components|GetOwner) "/Game/OpenRPG_Stats/Blueprints/Components/BPC_Attributes.BPC_Attributes_C"))
  (bind _success_ (Save/Load|LoadLevelingData))
  (if _success_
    (UI|InitializeWidgets)))

(event Custom|UpdateLevel
  (params (NewLevel :type Integer))
  ;[0.06453 0.8803 1] Leveling
  (for _array_element (Variables|UI|GetWidgets)
    (Class|BPILeveling|UpdateDisplayedLevel(Message) _array_element NewLevel)))

(event Custom|UpdateExperience
  (params (CurrentExperience :type Integer) (NeededExperience :type Integer) (TotalExperience :type Integer))
  ;[0.06453 0.8803 1] Leveling
  (for _array_element (Variables|UI|GetWidgets)
    (Class|BPILeveling|UpdateDisplayedExperience(Message) _array_element CurrentExperience NeededExperience TotalExperience)))

(fn ReceiveExperience
  (params (Experience :type Integer))
  (LocalVariables|SetLocalReceivedAmount Experience)
  (Variables|General|SetTotalExperience (+ (Variables|General|GetTotalExperience) (LocalVariables|GetLocalReceivedAmount)))
  (bind _output_get (Variables|General|SetCurrentExperience (+ (Variables|General|GetCurrentExperience) (LocalVariables|GetLocalReceivedAmount))))
  (while (>= _output_get (Variables|General|GetNeededExperience))
    (Variables|General|SetCurrentExperience (- (Variables|General|GetCurrentExperience) (Variables|General|GetNeededExperience))))
  (CallFunction|UpdateExperience (Variables|General|GetCurrentExperience) (Variables|General|GetNeededExperience) (Variables|General|GetTotalExperience))
  (Default|CallOnExperienceReceived (LocalVariables|GetLocalReceivedAmount) (Variables|General|GetCurrentExperience) (Variables|General|GetNeededExperience) (Variables|General|GetTotalExperience))
  (return))

(fn UpdateNeededExperience
  (params (NewLevel :type Integer))
  (LocalVariables|SetLocalLevel NewLevel)
  (if (Variables|Internal|GetUseCustomExperienceFormula?)
    (CallFunction|ExperienceFormula (LocalVariables|GetLocalLevel))
    (return)
    (elif (.ReturnValue (Utilities|Map|Find (Variables|Internal|GetNeededExperiencePerLevel) (LocalVariables|GetLocalLevel)))
      (Variables|General|SetNeededExperience (.Value (Utilities|Map|Find (Variables|Internal|GetNeededExperiencePerLevel) (LocalVariables|GetLocalLevel))))
      (return)
      (else
        (return)))))

(fn LevelUp
  (bind _output_get (Variables|General|SetCurrentLevel (+ (Variables|General|GetCurrentLevel) 1)))
  (if (== _output_get (Variables|Internal|GetMaxLevel))
    _
    (else
      (Managment|UpdateNeededExperience (Variables|General|GetCurrentLevel))))
  (CallFunction|ReceiveLevelUpReward (Variables|General|GetCurrentLevel))
  (Default|CallOnLevelUp (Variables|General|GetCurrentLevel))
  (CallFunction|UpdateLevel (Variables|General|GetCurrentLevel))
  (return))

(fn InitializeWidgets
  (CallFunction|UpdateLevel (Variables|General|GetCurrentLevel))
  (CallFunction|UpdateExperience (Variables|General|GetCurrentExperience) (Variables|General|GetNeededExperience) (Variables|General|GetTotalExperience))
  (return))

(fn AddCustomWidgets
  (params (Widgets :type Array%20of%20User%20Widget%20Object%20References))
  (for _array_element Widgets
    (Utilities|Array|AddUnique (Variables|UI|GetWidgets) _array_element))
  (return))

(fn LoadLevelingTableData
  (bind _returnvalue (Utilities|GetDataTableRow (Variables|Settings|GetLevelingTable) (Variables|Settings|GetLevelingTableRow))
    (:then
      (bind _output_get (LocalVariables|SetLocalLevelingData _returnvalue))
      (Variables|Internal|SetMaxLevel (.MaxLevel (Utilities|Struct|Breaks_Leveling _output_get)))
      (Variables|Internal|SetUseCustomExperienceFormula? (.UseCustomExperienceFormula? (Utilities|Struct|Breaks_Leveling _output_get)))
      (Variables|Internal|SetNeededExperiencePerLevel (.NeededExperiencePerLevel (Utilities|Struct|Breaks_Leveling _output_get)))
      (Variables|Internal|SetLevelRewards (.LevelRewards (Utilities|Struct|Breaks_Leveling _output_get)))
      (bind _keys (Utilities|Map|Keys (Variables|Internal|GetNeededExperiencePerLevel)))
      (bind _output_get_2 (Variables|Internal|SetStartingLevel (.MinValue (Math|Integer|MinOfIntArray _keys))))
      (Variables|General|SetCurrentLevel _output_get_2)
      (return true))
    (:RowNotFound
      (return false))))

(fn CreateLevelingSaveData
  (return (Utilities|Struct|Makes_LevelingSaveData (Variables|General|GetCurrentLevel) (Variables|General|GetCurrentExperience) (Variables|General|GetNeededExperience) (Variables|General|GetTotalExperience))))

(fn SaveLevelingData
  (bind _output_get (Variables|Save/Load|SetStatsSaveObject (CallFunction|GetStatsSaveObject (Variables|Save/Load|GetStatsSaveSlot))))
  (Utilities|IsValid _output_get
    (:Is%20Valid
      (Default|AddLevelingData (Variables|Save/Load|GetStatsSaveObject) (Variables|Settings|GetSaveName) (Save/Load|CreateLevelingSaveData))
      (bind _returnvalue (SaveGame|SaveGametoSlot (Variables|Save/Load|GetStatsSaveObject) (Variables|Save/Load|GetStatsSaveSlot)))
      (return _returnvalue))
    (:Is%20Not%20Valid
      (return false))))

(fn LoadLevelingData
  (bind _success_ (Save/Load|LoadLevelingTableData))
  (if _success_
    (bind _output_get (Variables|Save/Load|SetStatsSaveObject (CallFunction|GetStatsSaveObject (Variables|Save/Load|GetStatsSaveSlot))))
    (Utilities|IsValid _output_get
      (:Is%20Valid
        (if (.Found? (Default|GetLevelingData (Variables|Save/Load|GetStatsSaveObject) (Variables|Settings|GetSaveName)))
          (bind _output_get_2 (LocalVariables|SetLocalLevelingData (.LevelingData (Default|GetLevelingData (Variables|Save/Load|GetStatsSaveObject) (Variables|Settings|GetSaveName)))))
          (Variables|General|SetCurrentLevel (.CurrentLevel (Utilities|Struct|Breaks_LevelingSaveData _output_get_2)))
          (Variables|General|SetCurrentExperience (.CurrentExperience (Utilities|Struct|Breaks_LevelingSaveData _output_get_2)))
          (Variables|General|SetNeededExperience (.NeededExperience (Utilities|Struct|Breaks_LevelingSaveData _output_get_2)))
          (Variables|General|SetTotalExperience (.TotalExperience (Utilities|Struct|Breaks_LevelingSaveData _output_get_2)))
          (return true)
          (else
            (return false))))
      (:Is%20Not%20Valid
        (return false)))
    (else
      (return false))))
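; BPC_EnemyStats is a child stats component for demo enemies that limits enemy widget updates to the currently selected enemy.
; BP_DemoEnemy toggles a selection flag through select and deselect events, and selection immediately pushes a stat value and the level.
; An override of UpdateStatValue forwards to the parent only while selected.
; Initialize runs the parent setup, then applies a long ticking effect with a healing icon to test widget updates.
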(event `OnOwnerSelected`
  (bind (_value _currentvalue) (`self.GetStatValue` "NewEnumerator0"))
  ;[1 0.3217 0.1146] Called from the BP_DemoEnemy whenever its selected with the mouse. It sets the IsOwnerSelected boolean to true, so only the component with this boolean set to true will be able to update the widget
  (set `self.IsOwnerSelected?` true)
  (`self.UpdateStatValue` "NewEnumerator0" _value _currentvalue)
  (`self.UpdateLevel` (`self.CurrentLevel`)))

(event `OnOwnerSelectionRemoved`
  ;[1 0.3217 0.1146] Called from the BP_DemoEnemy when its no more selected
  (set `self.IsOwnerSelected?` false))

(event `self.UpdateStatValue`
  (params (Stat :type "/Game/OpenRPG_Stats/Enums/e_Stat Enum" :default "NewEnumerator7") (FinalValue :type "Float (single-precision)") (CurrentValue :type "Float (single-precision)"))
  ;[0.6115 1 0.1235] Due to inheritance, its very easy to override some events with extra conditions, in this case we need it to avoid any enemy to update the enemy widget when any of it stats is modified, only the selected one will be able to do so
  (if (`self.IsOwnerSelected?`)
    (`parent.UpdateStatValue` Stat FinalValue CurrentValue)))

(event `self.Initialize`
  (`parent.Initialize`)
  (`self.ApplyEffect` "NewEnumerator4" (make `/Game/OpenRPG_Stats/Structs/s_Effect` "/Game/Demo/Icons/Healing.Healing" 20.0 2000 1.0)) ; Just to check that the enemy widget updates correctly
)
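; Player stats component for an RPG that saves and loads stats, attributes, level and experience through a SaveStats save game slot.
; Initialize tries to load saved data, falls back to actor default data, then sets up widgets.
; Data is packed into one struct stored under SaveName within the slot's save object.
; Buffs and effects persist optionally, refreshing remaining times before saving and recomputing their shortest timers on load.
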(event `self.Initialize`
  (bind _success_ (`self.LoadStats`))
  (if (not _success_)
    (`self.LoadActorDefaultData`))
  (`self.InitializeWidgets`))

(fn `CreateStatsSaveData`
  (returns (Data :type "/Game/OpenRPG_Stats/Structs/s_SavedData Structure"))
  (locals (LocalDataToSave :type "/Game/OpenRPG_Stats/Structs/s_SavedData Structure"))
  (set `local.LocalDataToSave` (make `/Game/OpenRPG_Stats/Structs/s_SavedData` :`SavedStats` (`self.Stats`) :`SavedAttributes` (`self.Attributes`) :`SavedAttributeBonusesToStats` (`self.AttributeBonusesToStats`) :`SavedAttributesPerLevel` (`self.AttributesPerLevel`) :`SavedStatsPerLevel` (`self.StatsPerLevel`) :`SavedCurrentStats` (`self.CurrentStats`) :`SavedAvailableAttributePoints` (`self.AvailableAttributePoints`) :`SavedSpentAttributePoints` (`self.SpentAttributePoints`) :`SavedLevel` (`self.CurrentLevel`) :`SavedCurrentExperience` (`self.CurrentExperience`) :`SavedNeededExperienceToLevelUp` (`self.NeededExperienceToLevelUp`) :`SavedTotalExperience` (`self.TotalExperience`)))
  (if (`self.SaveBuffs?`)
    (`self.UpdateBuffsRemainingTime`)
    (bind _structout (setmembers `/Game/OpenRPG_Stats/Structs/s_SavedData` :`StructRef` (`local.LocalDataToSave`) :`SavedBuffs` (`self.Buffs`)))
    (set `local.LocalDataToSave` _structout))
  (if (`self.SaveEffects?`)
    (`self.UpdateEffectsRemainingIntervalTime`)
    (bind _structout_2 (setmembers `/Game/OpenRPG_Stats/Structs/s_SavedData` :`StructRef` (`local.LocalDataToSave`) :`SavedEffects` (`self.Effects`)))
    (set `local.LocalDataToSave` _structout_2))
  (return (`local.LocalDataToSave`)))

(fn `LoadStats`
  (returns (`Success?` :type Boolean))
  (locals (LocalSavedData :type "/Game/OpenRPG_Stats/Structs/s_SavedData Structure"))
  (bind ((`SavedAttributeBonusesToStats_53_BC1E31AC4D9B9B8A41EE6590A7D5E3AD` _savedattributebonusestostats) (`SavedAttributesPerLevel_46_BDCBD6D448FE5726DE9B82B6DC940D88` _savedattributesperlevel)) (break `/Game/OpenRPG_Stats/Structs/s_SavedData` (`local.LocalSavedData`)))
  (bind ((`SavedStatsPerLevel_51_B86956CA44F2B94921FA3FB2632A8781` _savedstatsperlevel) (`SavedCurrentStats_52_513C72F346D4966CF3C7F09E49A44B28` _savedcurrentstats)) (break `/Game/OpenRPG_Stats/Structs/s_SavedData` (`local.LocalSavedData`)))
  (bind ((`SavedAvailableAttributePoints_26_C56DCE3A41AB4654533C668F458C9D58` _savedavailableattributepoints) (`SavedSpentAttributePoints_27_DC23441541F244B50A25729137C785DD` _savedspentattributepoints)) (break `/Game/OpenRPG_Stats/Structs/s_SavedData` (`local.LocalSavedData`)))
  (bind ((`SavedLevel_18_9F222BBD41EE6146AD169A8DE399F4B3` _savedlevel) (`SavedCurrentExperience_20_169F37F24E53C4945FE1AEAAAC6D2D81` _savedcurrentexperience) (`SavedNeededExperienceToLevelUp_22_423C7AA744C70940D21B8CBAD98338CC` _savedneededexperiencetolevelup) (`SavedTotalExperience_28_7E821E624801EEB597D9EEA3A2A36474` _savedtotalexperience)) (break `/Game/OpenRPG_Stats/Structs/s_SavedData` (`local.LocalSavedData`)))
  (bind (_found_ _data) (`/Game/OpenRPG_Stats/Blueprints/SaveStats.GetStatsData` (`self.StatsSaveObject`) (`self.SaveName`)))
  (bind _success_ (`self.UpdateSaveObject` false))
  (if _success_
    (if _found_
      (bind _output_get (set `local.LocalSavedData` _data))
      (bind ((`SavedStats_31_BCBCF8324D7CD224253D489198C178A0` _savedstats) (`SavedAttributes_34_14AF42D74206AAB7399C3E80BDC9C9F7` _savedattributes)) (break `/Game/OpenRPG_Stats/Structs/s_SavedData` _output_get))
      (set `self.Stats` _savedstats)
      (set `self.Attributes` _savedattributes)
      (set `self.AttributeBonusesToStats` _savedattributebonusestostats)
      (set `self.AttributesPerLevel` _savedattributesperlevel)
      (set `self.StatsPerLevel` _savedstatsperlevel)
      (set `self.CurrentStats` _savedcurrentstats)
      (set `self.AvailableAttributePoints` _savedavailableattributepoints)
      (set `self.SpentAttributePoints` _savedspentattributepoints)
      (set `self.CurrentLevel` _savedlevel)
      (set `self.CurrentExperience` _savedcurrentexperience)
      (set `self.NeededExperienceToLevelUp` _savedneededexperiencetolevelup)
      (set `self.TotalExperience` _savedtotalexperience)
      (if (`self.SaveBuffs?`)
        (set `self.Buffs` (`.SavedBuffs_37_C8B1AB1240970074102EA78202C30666` (break `/Game/OpenRPG_Stats/Structs/s_SavedData` (`local.LocalSavedData`))))
        (`self.UpdateShortestBuffDuration`))
      (if (`self.SaveEffects?`)
        (set `self.Effects` (`.SavedEffects_40_1485022E43954BCEC46F8DA684C0FA72` (break `/Game/OpenRPG_Stats/Structs/s_SavedData` (`local.LocalSavedData`))))
        (`self.UpdateShortestEffectRemainingInterval`))
      (`self.OnStatsLoaded`)
      (return true)
      (else
        (return false)))
    (else
      (return false))))

(fn `SaveStats`
  (returns (`Success?` :type Boolean))
  (bind _success_ (`self.UpdateSaveObject` true))
  (if _success_
    (`/Game/OpenRPG_Stats/Blueprints/SaveStats.AddStatsData` (`self.StatsSaveObject`) (`self.SaveName`) (`self.CreateStatsSaveData`))
    (bind _returnvalue (`GameplayStatics.SaveGameToSlot` (`self.StatsSaveObject`) (`self.StatsSaveSlot`)))
    (if _returnvalue
      (`self.OnStatsSaved`)
      (return true)
      (else
        (return false)))
    (else
      (return false))))

(fn `UpdateSaveObject`
  (params (`Save?` :type Boolean))
  (returns (`Success?` :type Boolean))
  (locals (LocalSave :type Boolean))
  (set `local.LocalSave` `Save?`)
  (bind _returnvalue (`GameplayStatics.DoesSaveGameExist` (`self.StatsSaveSlot`)))
  (if _returnvalue
    (bind _returnvalue_2 (`GameplayStatics.LoadGameFromSlot` (`self.StatsSaveSlot`)))
    (bind _assave_stats (cast `/Game/OpenRPG_Stats/Blueprints/SaveStats` _returnvalue_2)
      (:`then`
        (set `self.StatsSaveObject` _assave_stats)
        (return true))
      (:`CastFailed`
        (return false)))
    (elif (`local.LocalSave`)
      (bind _returnvalue_3 (`GameplayStatics.CreateSaveGameObject` "/Game/OpenRPG_Stats/Blueprints/SaveStats.SaveStats_C"))
      (set `self.StatsSaveObject` _returnvalue_3)
      (return true)
      (else
        (return false)))))